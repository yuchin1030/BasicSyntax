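; BP_Actor06 is an Actor Blueprint that converts a Score variable into a letter grade and prints it.
; On BeginPlay, a chain of nested branches checks Score against descending thresholds and prints the matching grade from A down to F.
; The construction script is empty.
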(event EventBeginPlay
  (bind _score (Variables|Default|GetScore))
  (if (>= _score 90)
    (Development|PrintString "A")
    (elif (>= _score 80)
      (Development|PrintString "B")
      (elif (>= _score 70)
        (Development|PrintString "C")
        (elif (>= _score 60)
          (Development|PrintString "D")
          (else
            (Development|PrintString "F")))))))

(fn ConstructionScript)