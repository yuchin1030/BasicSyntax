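; BP_Actor04 is a small test actor that sums a range of integers and prints the results on screen.
; On BeginPlay it calls SumTotal from 3 to 7 and prints the returned total.
; SumTotal loops from the start to the end number, adding each index to the Number variable and printing each running subtotal.
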(event EventBeginPlay
  (bind _output (CallFunction|SumTotal 3 7))
  (Development|PrintString (Utilities|String|ToString(Integer) _output)))

(fn ConstructionScript)

(fn SumTotal
  (params (StartNumber :type Integer) (EndNumber :type Integer))
  ;[1 1 1] - this->number = number
  ; Start Number - First Index
  ; End Number - Last Index
  (for _index (range StartNumber EndNumber)
    (bind _output_get (Variables|Default|SetNumber (+ (Variables|Default|GetNumber) _index)))
    ;[1 1 1] 누계
    (Development|PrintString (Utilities|String|ToString(Integer) _output_get)))
  ;[1 1 1] 합계
  (return (Variables|Default|GetNumber)))