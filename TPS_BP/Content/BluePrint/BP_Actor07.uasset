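; BP_Actor07 is an actor that works out a clock end time from a start hour, minute and duration in minutes, apparently as a scripting exercise.
; On BeginPlay, EndTime runs with fixed inputs, carries minute overflow into hours, and wraps the hour past midnight with a single subtraction of 24.
; PrintTime then prints the resulting hour and minute on screen.
; An unconnected alternative version of the calculation remains in EndTime.
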(event EventBeginPlay
  (CallFunction|EndTime 23 48 25))

(fn ConstructionScript)

(fn EndTime
  (params (Hour :type Integer) (Minute :type Integer) (Time :type Integer))
  (Variables|Default|SetHour Hour)
  (bind _output_get (Variables|Default|SetMinute Minute))
  (bind _output_get_2 (Variables|Default|SetTime Time))
  (if (>= (+ _output_get _output_get_2) 60)
    (Variables|Default|SetHour (+ (/ (+ (Variables|Default|GetMinute) (Variables|Default|GetTime)) 60) (Variables|Default|GetHour)))
    (Variables|Default|SetMinute (Math|Integer|%(Integer) (+ (Variables|Default|GetMinute) (Variables|Default|GetTime)) 60))
    (if (>= (Variables|Default|GetHour) 24)
      (Variables|Default|SetHour (- (Variables|Default|GetHour) 24)))
    (CallFunction|PrintTime (Variables|Default|GetHour) (Variables|Default|GetMinute))
    (else
      (bind _output_get_3 (Variables|Default|SetMinute (+ (Variables|Default|GetMinute) (Variables|Default|GetTime))))
      (CallFunction|PrintTime (Variables|Default|GetHour) _output_get_3))))

(fn PrintTime
  (params (EndHour :type Integer) (EndMinute :type Integer))
  (Development|PrintString (Utilities|String|ToString(Integer) EndHour))
  (Development|PrintString (Utilities|String|ToString(Integer) EndMinute)))