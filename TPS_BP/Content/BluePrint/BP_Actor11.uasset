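; Test actor that prints a five-row star triangle to the screen on BeginPlay, apparently a nested-loop exercise.
; An outer loop builds each row from a padding string and a growing run of asterisks, prints them joined, then clears both.
; The padding appends empty strings, so it adds no indentation.
; An unconnected second version builds the same rows in one string using a branch inside the inner loop.
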(event EventBeginPlay
  (for _index (range 1 5)
    (for _index_2 (range 1 (- 5 _index))
      (bind _output_get (Variables|Default|SetBlank (Utilities|String|Append (Variables|Default|GetBlank) " "))))
    (for _index_3 (range 1 _index)
      (bind _output_get_2 (Variables|Default|SetStar (Utilities|String|Append (Variables|Default|GetStar) "*"))))
    (Development|PrintString (Utilities|String|Append _output_get _output_get_2) true true "(R=0.000000,G=0.660000,B=1.000000,A=1.000000)" 1e+01)
    (Variables|Default|SetBlank "")
    (Variables|Default|SetStar "")))

(fn ConstructionScript)