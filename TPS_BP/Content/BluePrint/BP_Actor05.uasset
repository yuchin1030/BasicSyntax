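; BP_Actor05 is an actor that scores a three-dice roll and prints the result, evaluating one hard-coded roll on BeginPlay.
; The Dice function branches on whether all three values match, exactly two match or all differ, passing the matched or highest value to one of three print helpers.
; Each helper applies its own prize formula, with larger payouts for more matching dice.
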(event EventBeginPlay
  (CallFunction|Dice 6 2 5))

(fn ConstructionScript)

(fn Dice
  (params (Dice01 :type Integer) (Dice02 :type Integer) (Dice03 :type Integer))
  (Variables|Default|SetDice1 Dice01)
  (Variables|Default|SetDice2 Dice02)
  (Variables|Default|SetDice3 Dice03)
  ;[1 1 1] if : 3개 모두 같은 경우
  (if (and (== (Variables|Default|GetDice1) (Variables|Default|GetDice2)) (== (Variables|Default|GetDice2) (Variables|Default|GetDice3)))
    (CallFunction|PrintEqualThree (Variables|Default|GetDice1))
    (else
      ;[1 1 1] else if : 2개만 같은 경우
      (if (== (Variables|Default|GetDice1) (Variables|Default|GetDice2))
        (CallFunction|PrintEqualTwo (Variables|Default|GetDice1))
        (elif (== (Variables|Default|GetDice2) (Variables|Default|GetDice3))
          (CallFunction|PrintEqualTwo (Variables|Default|GetDice2))
          (elif (== (Variables|Default|GetDice3) (Variables|Default|GetDice1))
            (CallFunction|PrintEqualTwo (Variables|Default|GetDice3))
            (else
              ;[1 1 1] else : 3개 모두 다른 경우
              (CallFunction|PrintDifferent (Math|Integer|Max(Integer) (Variables|Default|GetDice1) (Variables|Default|GetDice2) (Variables|Default|GetDice3))))))))))

(fn PrintEqualThree
  (params (Dice1 :type Integer))
  (Development|PrintString (Utilities|String|ToString(Integer) (+ (* Dice1 1000) 10000))))

(fn PrintEqualTwo
  (params (Dice :type Integer))
  (Development|PrintString (Utilities|String|ToString(Integer) (+ (* Dice 100) 1000))))

(fn PrintDifferent
  (params (Max :type Integer))
  (Development|PrintString (Utilities|String|ToString(Integer) (* Max 100))))