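; Prototype pickup actor that can follow in front of the player and dissolve away.
; While IsPlayer is true, Tick snaps it ahead of the player character; a sphere hit from that character clears the flag.
; PickedUP, not called within this Blueprint, plays a timeline driving a dynamic dissolve material through DynaMatChange, then destroys the actor.
; An attach-to-actor alternative is left unconnected.
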(event OnComponentHit(Sphere1)
  (params (HitComponent :type Primitive%20Component%20Object%20Reference) (OtherActor :type Actor%20Object%20Reference) (OtherComp :type Primitive%20Component%20Object%20Reference) (NormalImpulse :type Vector :default "0, 0, 0") (Hit :type Hit%20Result%20Structure%20%28by%20ref%29))
  (bind _asbp_third_person_character (Utilities|Casting|CastToBP_ThirdPersonCharacter (Game|GetPlayerCharacter 0))) ; 부딪힌 대상
  (if (== OtherActor _asbp_third_person_character)
    (Variables|Default|SetisPlayer false)))

(event Custom|FollowUp
  (bind _returnvalue (Game|GetPlayerCharacter 0))
  ;[1 1 1] 나(픽업오브젝트,self)의 위치를 업데이트 해라
  (Transformation|SetActorLocation (+ (Transformation|GetActorLocation _returnvalue) (* (Transformation|GetActorForwardVector _returnvalue) 105.0)) false false))

(event EventBeginPlay
  ;[1 1 1] I will change to parameter in Material
  (bind _returnvalue (Rendering|Material|CreateDynamicMaterialInstance (Variables|Default|GetSphere) 0 "/Game/Proto/Materials/MI_dissolve.MI_dissolve" "None" :!class /Script/Engine.PrimitiveComponent))
  (Variables|Default|SetdissolveMat _returnvalue)
  (Utilities|DynaMatChange 1.0 0.0 0.0))

(event EventPickedUP
  ;[1 1 1] 히트 된 대상(other)가 플레이어라면
  (bind _dissolve (Timeline|dyMatTimeLine Play)
    (:Update
      (Utilities|DynaMatChange _dissolve 0.1 1e+01))
    (:Finished
      (Actor|DestroyActor))))

(event EventTick
  (params (DeltaSeconds :type Float%20%28single-precision%29))
  ;[1 1 1] 플레이어의 정면 방향을 받아온다
  (if (Variables|Default|GetisPlayer) ; 플레이어가 픽없했을때만
    (CallFunction|FollowUp)))

(fn ConstructionScript)