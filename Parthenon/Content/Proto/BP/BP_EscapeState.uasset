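; Tracks the time limit and dial-puzzle completion for a prototype escape game.
; BeginPlay sizes a boolean array to the level's BP_DialManager count; each CheckDialManager call flags the first unsolved slot, finishing when all are true.
; Outside sequence playback, Tick updates UI_Timer's ratio and text until time expires, then adds UI_Result every frame while finished.
; TimerInit creates the timer widget; its opening-sequence check is disconnected.
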(event Custom|ProgUpdate
  ;[1 1 1] 부분/전체 : cur / limit = 비율
  (Variables|/Game/Proto/UI/UI_Timer.UI_Timer_C|SetTimeRatio (Variables|Default|GetuiTimerRef) (/ (Variables|Default|GetcurTime) (Variables|Default|GetlimitTime))))

(event Custom|Time%20TextUpdate
  (bind _curtime (Variables|Default|GetcurTime))
  ;[1 1 1] UI time text update
  (Variables|/Game/Proto/UI/UI_Timer.UI_Timer_C|SetTimeText (Variables|Default|GetuiTimerRef) (Utilities|Text|FormatText "{min} : {sec}" (Utilities|Text|ToText(Float) (/ _curtime 6e+01) "ToZero" false true 2 2 0 0) (Utilities|Text|ToText(Float) (Math|Float|%(Float) _curtime 6e+01) "ToZero" false true 2 2 0 0))))

(event Custom|TimerInit
  (if (not (Variables|Default|GetisSequencePlay))
    (Variables|Default|SetcurTime 0.0) ; 시간 초기화(initialize)
    (bind _returnvalue (UserInterface|CreateWidget "/Game/Proto/UI/UI_Timer.UI_Timer_C")) ; 위젯 만들자마자
    (bind _output_get (Variables|Default|SetuiTimerRef _returnvalue)) ; 변수 만들고 설정해놓기
    (UserInterface|Viewport|AddtoViewport _output_get 0)))

(event Custom|CheckDialManager
  ;[1 1 1] (특정 1개의) DialManager가 해결됐냐 (선착순 - but 문제많음)
  (bind (_array_element _array_index) (Utilities|Array|ForEachLoopwithBreak (Variables|Default|GetisDialManagerCheck) :!label _label)
    (:LoopBody
      (if (not _array_element)
        (Utilities|Array|SetArrayElem (Variables|Default|GetisDialManagerCheck) _array_index true)
        (goto _label Break)))
    (:Completed
      (CallFunction|CheckClear))))

(event Custom|CheckClear
  (if (not (Utilities|Array|ContainsItem (Variables|Default|GetisDialManagerCheck) false)) ; True : not clear // False : clear
    (Variables|Default|SetisFinished true)))

(event EventBeginPlay
  (bind _isdialmanagercheck (Variables|Default|GetisDialManagerCheck))
  ;[1 1 1] 현재 레벨에 배치된 DialManager 개수만큼 배열 길이를 set
  (bind _outactors (Actor|GetAllActorsOfClass "/Game/Proto/BP/BP_DialManager.BP_DialManager_C"))
  (Utilities|Array|Resize _isdialmanagercheck (Utilities|Array|Length _outactors))
  (Development|PrintString (Utilities|String|ToString(Integer) (Utilities|Array|Length _isdialmanagercheck))))

(event EventTick
  (params (DeltaSeconds :type Float%20%28single-precision%29))
  ;[1 1 1] Timer  시간 안에 클리어 했는지 (True : Limit Time Over // False : Playing)
  (if (not (Variables|Default|GetisSequencePlay))
    (if (Variables|Default|GetisFinished)
      (bind _returnvalue (UserInterface|CreateWidget "/Game/Proto/UI/UI_Result.UI_Result_C" :!label _label))
      (UserInterface|Viewport|AddtoViewport _returnvalue 0)
      (Variables|Default|SetisFinished true)
      (else
        (bind _output_get (Variables|Default|SetcurTime (+ DeltaSeconds (Variables|Default|GetcurTime)))) ; 현재 값 + delta seconds ==> 누적
        (if (>= _output_get (Variables|Default|GetlimitTime)) ; True : Game over // False : Playing
          (goto _label)
          (else
            (CallFunction|ProgUpdate)
            (CallFunction|TimeTextUpdate)))))))

(fn ConstructionScript)