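; BP_DialManager is a combination-dial puzzle that checks the dials against a password and reports the solve to BP_EscapeState.
; Its construction script spawns a vertical stack of child-actor dials, one per password entry.
; GetDialsCurNum compares each dial's number to the password, and PasswordChecker fires AnswerAllTrue and locks the solved state when all match.
; Player overlap with the capsule sets IsDial, blends the view to the manager and shows the cursor.
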(event OnComponentBeginOverlap(Capsule)
  (params (OverlappedComponent :type Primitive%20Component%20Object%20Reference) (OtherActor :type Actor%20Object%20Reference) (OtherComp :type Primitive%20Component%20Object%20Reference) (OtherBodyIndex :type Integer) (bFromSweep :type Boolean) (SweepResult :type Hit%20Result%20Structure%20%28by%20ref%29))
  (bind _returnvalue (Game|GetPlayerController 0))
  (if (== OtherActor (Game|GetPlayerCharacter 0))
    (bind _asbp_third_person_character (Utilities|Casting|CastToBP_ThirdPersonCharacter OtherActor))
    (Variables|/Game/ThirdPerson/Blueprints/BP_ThirdPersonCharacter.BP_ThirdPersonCharacter_C|SetisDial _asbp_third_person_character true)
    (Game|Player|SetViewTargetwithBlend _returnvalue self 2.0 "VTBlend_Linear" 0.0 false)
    (Variables|/Script/Engine.PlayerController|SetbShowMouseCursor _returnvalue true)))

(event Custom|PasswordChecker
  ;[1 1 1] 정답을 확인한다 == answerArr
  (if (Utilities|Array|ContainsItem (Variables|Default|GetanswerArr) false) ; True : Wrong // False : Correct
    (Development|PrintString "Wrong")
    (else
      (Development|PrintString "Correct")
      (Default|CallAnswerAllTrue)
      (Variables|Default|SetisSolved true)
      (bind _asbp_escape_state (Utilities|Casting|CastToBP_EscapeState (Game|GetGameState)))
      (Default|CheckDialManager _asbp_escape_state))))

(event Custom|GetDialsCurNum
  (bind _answerarr (Variables|Default|GetanswerArr))
  (if (not (Variables|Default|GetisSolved))
    ;[1 1 1] Child BP_Dial의 curNum를 가지고 온다
    (for (_ _array_index) (Variables|Default|GetpasswordArr)
      (bind _asbp_dial (Utilities|Casting|CastToBP_Dial (Variables|/Script/Engine.ChildActorComponent|GetChildActor (Utilities|Array|Get(acopy) (Variables|Default|GetdialArr) _array_index))))
      ;[1 1 1] curNum와 passwordArr를 비교한다
      (if (== (Variables|/Game/Proto/Password/BP_Dial.BP_Dial_C|GetcurNum _asbp_dial) (Utilities|Array|Get(acopy) (Variables|Default|GetpasswordArr) _array_index)) ; True : Match // False : Not matched
        ;[1 1 1] 비교한 결과를 answerArr에 저장
        (Utilities|Array|SetArrayElem _answerarr _array_index true)
        (else
          (Utilities|Array|SetArrayElem _answerarr _array_index false))))
    (CallFunction|PasswordChecker)))

(fn ConstructionScript
  (bind _passwordarr (Variables|Default|GetpasswordArr))
  (bind _answerarr (Variables|Default|GetanswerArr))
  (bind _returnvalue (Utilities|Array|Length _passwordarr))
  (Utilities|Array|Clear _answerarr)
  (Utilities|Array|Resize _answerarr _returnvalue) ; if 4 : 0~3
  (Utilities|Array|Clear (Variables|Default|GetdialArr))
  (for _index (range 0 (- _returnvalue 1))
    (bind _returnvalue_2 (AddComponent|AddChildActorComponent false (Math|Transform|MakeTransform (Variables|Default|GetdialLoc) "0, 0, 0" "1.000000,1.000000,1.000000")))
    (Utilities|Array|Add (Variables|Default|GetdialArr) _returnvalue_2)
    (Variables|Default|SetdialLoc (Math|Vector|MakeVector (.x (Variables|Default|GetdialLoc)) (.y (Variables|Default|GetdialLoc)) (+ (.z (Variables|Default|GetdialLoc)) -4e+01)))))