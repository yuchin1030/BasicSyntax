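; Prototype moving-object Blueprint that slides its Cube component back and forth along local X, between roughly 0 and 250 units.
; Each Tick offsets the relative X by Speed, with the Is boolean selecting direction and flipping at either limit.
; Movement is not scaled by delta time, so it depends on frame rate; it does not sweep and forces relative Y and Z to zero.
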(event EventTick
  (params (DeltaSeconds :type Float%20%28single-precision%29))
  (bind _cube (Variables|Default|GetCube))
  (bind _speed (Variables|Default|Getspeed))
  (bind _cube_2 (Variables|Default|GetCube))
  (bind _returnvalue (* _speed -1.0))
  (bind _returnvalue_2 (* _speed 1.0))
  (bind _relativelocation (Variables|/Script/Engine.SceneComponent|GetRelativeLocation _cube))
  (bind _relativelocation_2 (Variables|/Script/Engine.SceneComponent|GetRelativeLocation _cube_2))
  (bind _returnvalue_3 (+ (.x _relativelocation) _returnvalue))
  (bind _returnvalue_4 (+ (.x _relativelocation_2) _returnvalue_2))
  (if (Variables|Default|Getis)
    (Transformation|SetRelativeLocation (Variables|Default|GetCube) (Math|Vector|MakeVector _returnvalue_4 0.0 0.0) false false)
    (if (>= _returnvalue_4 2.5e+02)
      (Variables|Default|Setis false))
    (else
      (Transformation|SetRelativeLocation (Variables|Default|GetCube) (Math|Vector|MakeVector _returnvalue_3 0.0 0.0) false false)
      (if (<= _returnvalue_3 0.0)
        (Variables|Default|Setis true)))))

(event EventBeginPlay)

(fn ConstructionScript)