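; BP_TriggerBox is a prototype trigger actor that slides a gate mesh along Z as the player character enters and leaves.
; Begin overlap plays the GateSliding timeline and end overlap reverses it, both filtered to player pawn 0.
; Timeline updates add MoveZ times Speed to the gate's current relative Z rather than interpolating fixed positions, and Finished flips Speed's sign.
; Unconnected movement, rotation and event-binding experiments remain unused.
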(event OnComponentEndOverlap(Box)
  (params (OverlappedComponent :type Primitive%20Component%20Object%20Reference) (OtherActor :type Actor%20Object%20Reference) (OtherComp :type Primitive%20Component%20Object%20Reference) (OtherBodyIndex :type Integer)))

(event Custom|OnActorEndOverlap_Event
  (params (OverlappedActor :type Actor%20Object%20Reference) (OtherActor :type Actor%20Object%20Reference)))

(event EventBeginPlay)

(event Collision|EventActorBeginOverlap
  (params (OtherActor :type Actor%20Object%20Reference))
  (bind _sm_gate (Variables|Default|GetSM_Gate))
  (bind _relativelocation (Variables|/Script/Engine.SceneComponent|GetRelativeLocation _sm_gate))
  ;[1 1 1] 플레이어가 트리거 영역에 들어오면
  ;;[1 1 1] 생략 가능
  (bind _asbp_third_person_character (Utilities|Casting|CastToBP_ThirdPersonCharacter OtherActor))
  (Utilities|IsValid _asbp_third_person_character ; 유효성검사\n트리거 영역에 들어온게 ThirdPerson이 \n맞는지 다시 한 번 더 확인(데이터가 유효한지)
    (:Is%20Valid
      (if (== _asbp_third_person_character (Game|Player|GetPlayerPawn 0))
        ;[1 1 1] 문을 위에서 아래로 슬라이딩(이동)되라
        (bind _movez (Timeline|GateSliding Play)
          (:Update
            (Transformation|SetRelativeLocation _sm_gate (Math|Vector|MakeVector (.x _relativelocation) (.y _relativelocation) (+ (.z _relativelocation) (* _movez (Variables|Default|Getspeed)))) false false))
          (:Finished
            (Variables|Default|Setspeed (* (Variables|Default|Getspeed) -1.0))))))))

(event EventTick
  (params (DeltaSeconds :type Float%20%28single-precision%29)))

(event Collision|EventActorEndOverlap
  (params (OtherActor :type Actor%20Object%20Reference))
  (bind _sm_gate (Variables|Default|GetSM_Gate))
  (bind _relativelocation (Variables|/Script/Engine.SceneComponent|GetRelativeLocation _sm_gate))
  (bind _asbp_third_person_character (Utilities|Casting|CastToBP_ThirdPersonCharacter OtherActor))
  (Utilities|IsValid _asbp_third_person_character ; 유효성검사\n트리거 영역에 들어온게 ThirdPerson이 \n맞는지 다시 한 번 더 확인(데이터가 유효한지)
    (:Is%20Valid
      (if (== _asbp_third_person_character (Game|Player|GetPlayerPawn 0))
        ;[1 1 1] 문을 위에서 아래로 슬라이딩(이동)되라
        (bind _movez (Timeline|GateSliding Reverse)
          (:Update
            (Transformation|SetRelativeLocation _sm_gate (Math|Vector|MakeVector (.x _relativelocation) (.y _relativelocation) (+ (.z _relativelocation) (* _movez (Variables|Default|Getspeed)))) false false))
          (:Finished
            (Variables|Default|Setspeed (* (Variables|Default|Getspeed) -1.0))))))))

(fn ConstructionScript)