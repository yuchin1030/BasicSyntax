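; Rotating number dial for a password puzzle, run as a child actor of BP_DialManager.
; The construction script spaces Count numbered text labels and collision spheres evenly around the cylinder.
; Each PickedUP turns the cylinder one step, and a Checker overlap stores the matched sphere's index as CurNum, then calls the manager's GetDialsCurNum.
; The manager's AnswerAllTrue dispatcher sets IsCorrect, which locks further rotation.
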(event OnComponentBeginOverlap(Checker)
  (params (OverlappedComponent :type Primitive%20Component%20Object%20Reference) (OtherActor :type Actor%20Object%20Reference) (OtherComp :type Primitive%20Component%20Object%20Reference) (OtherBodyIndex :type Integer) (bFromSweep :type Boolean) (SweepResult :type Hit%20Result%20Structure%20%28by%20ref%29))
  ;[1 1 1] Array -> For - Break : Compare collArr with otherComp
  (bind (_array_element _array_index) (Utilities|Array|ForEachLoopwithBreak (Variables|Default|GetcollArr) :!label _label) ; break 걸었을 당시에 Completed 수행
    (:LoopBody
      (if (== _array_element OtherComp)
        (goto _label Break)))
    (:Completed
      (Variables|Default|SetcurNum _array_index) ; 현재 번호 저장
      (Default|GetDialsCurNum (Variables|Default|Getmanager)))))

(event Custom|FlipIsCorrect
  ;[1 1 1] Manager의 AnswerAllTrue(dispatcher) 가 호출되면 Bind 되어 있는 FlipIsCorrect도 같이 실행시켜
  (Variables|Default|SetisCorrect true))

(event EventPickedUP
  ;[1 1 1] 실린더를 회전시켜라
  (if (not (Variables|Default|GetisCorrect))
    (bind _output_get (Variables|Default|SetCylinderRot (Math|Rotator|MakeRotator (.roll (Variables|Default|GetCylinderRot)) (.pitch (Variables|Default|GetCylinderRot)) (+ (.yaw (Variables|Default|GetCylinderRot)) (Variables|Default|Getangle)))))
    (Transformation|SetRelativeRotation (Variables|Default|GetCylinder) _output_get false false)))

(event EventBeginPlay
  ;[1 1 1] 초기화
  (Variables|Default|SetCylinderRot (Variables|/Script/Engine.SceneComponent|GetRelativeRotation (Variables|Default|GetCylinder)))
  (Variables|Default|SetisCorrect false)
  (Variables|Default|Setangle (/ 3.6e+02 (Math|Conversions|ToFloat(Integer) (Variables|Default|Getcount))))
  ;[1 1 1] BP_DialMgager을 찾아라
  (bind _asbp_dial_manager (Utilities|Casting|CastToBP_DialManager (Actor|GetParentActor)))
  (bind _output_get (Variables|Default|Setmanager _asbp_dial_manager))
  ;[1 1 1] DailManager의 GetDialsCurNum을 실행
  (Default|GetDialsCurNum _output_get)
  ;[1 1 1] Manager의 AnswerAllTrue(dispatcher) 가 호출되면 Bind 되어 있는 FlipIsCorrect도 같이 실행시켜
  (EventDispatchers|BindEventtoAnswerAllTrue _output_get (delegate Custom|FlipIsCorrect)))

(fn ConstructionScript
  (Utilities|Array|Clear (Variables|Default|GetcollArr)) ; 배열 비우기\n(Construction에서 배열을 반복할때 꼭 해줘야함. \n안하면 배열이 계속 증식됨)
  (bind _returnvalue (|CountCalcDegree)) ; Collapse Node : 정리용
  ;[1 1 1] 반복
  (for _index (range 0 _returnvalue)
    ;[1 1 1] 반복한다
    ;;[1 1 1] Text Renderer Component를  배치한다
    ;; (Hierarchy엔 안보임)
    (bind _returnvalue_2 (AddComponent|AddTextRenderComponent false (Math|Transform|MakeTransform (* (Math|Vector|GetForwardVector (Variables|Default|GetarrRot)) 51.0) (Variables|Default|GetarrRot) "1.000000,1.000000,1.000000")))
    (Rendering|Components|TextRender|SetText _returnvalue_2 (Utilities|Text|ToText(Integer) _index))
    (Rendering|Components|TextRender|SetHorizontalAlignment _returnvalue_2 "EHTA_Center")
    (Class|TextRenderComponent|SetVerticalAlignment _returnvalue_2 "EVRTA_TextCenter")
    (Rendering|Components|TextRender|SetTextRenderColor _returnvalue_2 (Math|Color|MakeColor 0 0 255 255))
    (Transformation|AttachComponentToComponent _returnvalue_2 (Variables|Default|GetCylinder) "None" "KeepRelative" "KeepRelative" "KeepWorld" true)
    ;[1 1 1] Sphere Collision 추가
    (bind _returnvalue_3 (AddComponent|AddSphereComponent false (Math|Transform|MakeTransform (* (Math|Vector|GetForwardVector (Variables|Default|GetarrRot)) 57.0) "0, 0, 0" "1.000000,1.000000,1.000000")))
    (Utilities|Array|Add (Variables|Default|GetcollArr) _returnvalue_3) ; Item 추가
    (Transformation|AttachComponentToComponent _returnvalue_3 (Variables|Default|GetCylinder) "None" "KeepRelative" "KeepRelative" "KeepRelative" true)
    ;[1 1 1] Angle만큼 회전한다
    (Variables|Default|SetarrRot (Math|Rotator|MakeRotator (.roll (Variables|Default|GetarrRot)) (.pitch (Variables|Default|GetarrRot)) (+ (.yaw (Variables|Default|GetarrRot)) (Variables|Default|Getangle))))))